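; Player character that aims at the mouse and fights roots with a fuel-limited flamethrower.
; Firing toggles Niagara flames, light and sound, while looping timers drive fuel drain, Root Killer spawns at the detection point and regeneration on release.
; BeginPlay creates the timer, fuel and score HUD, and Escape or P toggles the pause menu.
; Touching BP_Roots plays death effects, saves, pauses and shows Game Over with the score.
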(event OnComponentBeginOverlap(CapsuleComponent)
  (params (OverlappedComponent :type Primitive%20Component%20Object%20Reference) (OtherActor :type Actor%20Object%20Reference) (OtherComp :type Primitive%20Component%20Object%20Reference) (OtherBodyIndex :type Integer) (bFromSweep :type Boolean) (SweepResult :type Hit%20Result%20Structure%20%28by%20ref%29))
  ;[0.3833 0.4599 1] When player collides with the roots the game over UI appears and pauses the game
  (Utilities|Casting|CastToBP_Roots OtherActor)
  (Audio|PlaySound2D "/Game/Sounds/GameSounds/DeathSound.DeathSound" 1.0 1.0 0.0 0 0)
  (Audio|PlaySound2D "/Game/Sounds/GameSounds/gameover.gameover" 1.7 1.0 0.0 0 0)
  (Niagara|SpawnSystematLocation "/Game/DeathParticle.DeathParticle" "0, 0, 0")
  (Components|DestroyComponent (Variables|Default|GetS_Player))
  (Niagara|SpawnSystematLocation "/Game/HellOnEarth/NS_RootsCrack.NS_RootsCrack" "0, 0, 0" "0, 0, 0" "1.000000,1.000000,1.000000" false)
  (SaveGame|SaveGametoSlot (Variables|Default|GetSaverSubClass) (Variables|/Game/Blueprints/Player/GM_Bogged.GM_Bogged_C|GetSave%20Slot%20Name (Variables|Default|GetAs%20GM%20Bogged)))
  (Game|SetGamePaused true)
  (bind _returnvalue (UserInterface|CreateWidget "/Game/Widgets/WBP_GameOver.WBP_GameOver_C"))
  (bind _output_get (Variables|Default|SetDeathWBP _returnvalue))
  (Variables|/Game/Widgets/WBP_GameOver.WBP_GameOver_C|SetGameOverScore _output_get (Variables|/Game/Blueprints/Player/GM_Bogged.GM_Bogged_C|GetNewScore (Variables|Default|GetAs%20GM%20Bogged)))
  (UserInterface|Viewport|AddtoViewport _returnvalue 0)
  (Variables|Default|SetIsDead true))

(event Custom|SpawnRK
  ;[0.6406 0.01083 0] "SpawnRK" is what handles the spawning of the Root Killer, use with caution
  (if (Variables|Default|GetIsFiring)
    (if (<= (Variables|Default|GetFuel) 0.0)
      (Components|Activation|Deactivate (Variables|Default|GetNS_Emitter))
      (else
        (Game|SpawnActorfromClass "/Game/HellOnEarth/BP_RootKiller.BP_RootKiller_C" (Transformation|GetWorldTransform (Variables|Default|GetRootDetection)) "AdjustIfPossibleButAlwaysSpawn" 0 0)))))

(event Custom|BeginFireSequence
  ;[1 0.491 0.07819] Handles the firing of the weapon, will deactivate if the weapon reaces 0, will continue to fire if the weapon can. Triggers the "Use Fuel" event.
  (if (<= (Variables|Default|GetFuel) 0.0)
    (Variables|Default|SetIsFiring false)
    (Rendering|Components|Light|SetIntensity (Variables|Default|GetPointLight) 0.0)
    (Variables|Default|SetStartRegain true)
    (Components|Activation|Deactivate (Variables|Default|GetNS_Emitter))
    (else
      (Variables|Default|SetIsFiring true)
      (Rendering|Components|Light|SetIntensity (Variables|Default|GetPointLight) 1.5e+04)
      (bind _returnvalue (Audio|SpawnSound2D "/Game/Sounds/GameSounds/FlameThrowerShoot.FlameThrowerShoot" 5.0 1.1 0.0 0))
      (bind _output_get (Variables|Default|SetFlameThrowerSound _returnvalue))
      (Components|Activation|SetActive _output_get true false)
      (Variables|Default|SetStartRegain false)
      (Components|Activation|Activate (Variables|Default|GetNS_Emitter) true)
      (CallFunction|UseFuel)
      (Utilities|Time|SetTimerbyEvent (EventDispatchers|CreateEvent :!event Custom|UseFuel) 0.5 true))))

(event Custom|UseFuel
  ;[1 0.4994 0.4895] This handles the use of the fuel, directly tied to the firing mechanic.
  (if (Variables|Default|GetIsFiring)
    (Variables|Default|SetStartRegain false)
    (Variables|Default|SetFuel (Math|Float|MapRangeClamped (- (Variables|Default|GetFuel) 5.0) 0.0 1e+02 0.0 1e+02))
    (else
      (Variables|Default|SetStartRegain true))))

(event Custom|RegainFuel
  ;[0.2582 1 0.2159] Begin RegainFuel event, this is called whenever we are stopping the firing of the weapon and features a cap on how much fuel we can get back (100).
  (if (Variables|Default|GetIsFiring)
    (Variables|Default|SetStartRegain false)
    (else
      (Variables|Default|SetStartRegain true)
      (if (not (== (Variables|Default|GetFuel) (Variables|Default|GetMaxFuel)))
        (Utilities|FlowControl|Delay (Variables|Default|GetRegainFuelRate))
        (bind _output_get (Variables|Default|SetFuel (Math|Float|MapRangeClamped (+ (Variables|Default|GetFuel) 5.0) 0.0 1e+02 0.0 1e+02)))
        (CallFunction|FuelInfo _output_get)))))

(event EventLookat
  (params (PlayerTarget :type Vector :default "0, 0, 0"))
  (bind _mesh (Variables|Character|GetMesh))
  (bind _returnvalue (Transformation|GetWorldLocation _mesh))
  ;[0.1305 0.06354 1] Makes player look at mouse.
  (Transformation|SetActorRotation (Math|Rotator|FindLookatRotation (Math|Vector|MakeVector (.x _returnvalue) (.y _returnvalue) 0.0) (Math|Vector|MakeVector (.x PlayerTarget) (.y PlayerTarget) 0.0))))

(event EventBeginPlay
  (bind _asgm_bogged (Utilities|Casting|CastToGM_Bogged (Game|GetGameMode)))
  (Variables|Default|SetAs%20GM%20Bogged _asgm_bogged)
  (bind _returnvalue (UserInterface|CreateWidget "/Game/Maps/Timer.Timer_C"))
  ;[0.377 1 0.7866] Sets fuel
  (Variables|Default|SetFuel (Variables|Default|GetMaxFuel))
  (bind _returnvalue_2 (UserInterface|CreateWidget "/Game/Blueprints/Player/WBP_FuelIndicator.WBP_FuelIndicator_C"))
  (bind _returnvalue_3 (UserInterface|CreateWidget "/Game/Widgets/WBP_NewScore.WBP_NewScore_C"))
  (UserInterface|Viewport|AddtoViewport _returnvalue_3 0))

(event Input|ActionEvents|InputActionFire
  (params (Key :type Key%20Structure :default "None"))
  (:Pressed
    ;[1 0.491 0.07819] The pressed input here will allow the "Begin Fire Sequence" & "Spawn RK" to trigger. Once this happens, it starts the timers respective of the events
    (CallFunction|BeginFireSequence)
    (CallFunction|SpawnRK)
    (Utilities|Time|SetTimerbyEvent (EventDispatchers|CreateEvent :!event Custom|SpawnRK) (Variables|Default|GetFireRate) true)
    (Utilities|Time|SetTimerbyEvent (EventDispatchers|CreateEvent :!event Custom|BeginFireSequence) 0.0 true))
  (:Released
    ;[0.2582 1 0.2159] This handles the stopping of the firing. Will begin the "Regain Fuel" event which trigger the timer.
    (Variables|Default|SetIsFiring false)
    (Components|Activation|Deactivate (Variables|Default|GetNS_Emitter))
    (Rendering|Components|Light|SetIntensity (Variables|Default|GetPointLight) 0.0)
    (Components|Activation|SetActive (Variables|Default|GetFlameThrowerSound) false false)
    (CallFunction|RegainFuel)
    (Utilities|Time|SetTimerbyEvent (EventDispatchers|CreateEvent :!event Custom|RegainFuel) 0.5 (Variables|Default|GetStartRegain))))

(event Input|KeyboardEvents|Escape
  (params (Key :type Key%20Structure :default "None"))
  (:Pressed
    (Utilities|FlowControl|FlipFlop
      (:A
        (Game|SetGamePaused true)
        (bind _returnvalue (UserInterface|CreateWidget "/Game/Widgets/WBP_Paused.WBP_Paused_C"))
        (UserInterface|Viewport|AddtoViewport _returnvalue 0))
      (:B
        (Game|SetGamePaused false)
        (Widget|RemovefromParent _returnvalue)))))

(event Input|KeyboardEvents|P
  (params (Key :type Key%20Structure :default "None"))
  (:Pressed
    (Utilities|FlowControl|FlipFlop
      (:A
        (Game|SetGamePaused true)
        (bind _returnvalue (UserInterface|CreateWidget "/Game/Widgets/WBP_Paused.WBP_Paused_C"))
        (UserInterface|Viewport|AddtoViewport _returnvalue 0))
      (:B
        (Game|SetGamePaused false)
        (Widget|RemovefromParent _returnvalue)))))

(fn ConstructionScript)

(fn FuelInfo
  (params (Current%20Fuel :type Float%20%28double-precision%29))
  (return 0.0))