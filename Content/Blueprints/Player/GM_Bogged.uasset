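; GM_Bogged is the game mode that tracks the player's score and carries it between levels.
; On BeginPlay it deletes the save slot in Level_1, otherwise loads the saved score, creating a save if none exists.
; EndPlay writes the score into a newly created GM_Bogged_SaveGame object and saves it to the slot.
; UpdateGMScore adds points for killed roots unless StopScoring is set.
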(event EventBeginPlay
  ;[1 1 1] Start of the GM, we delete any existing save or load into a pre-existing
  (bind _returnvalue (Game|GetCurrentLevelName true))
  (if (Utilities|Enum|Equal(Enum) _returnvalue "Level_1")
    (SaveGame|DeleteGameinSlot (Variables|Default|GetSave%20Slot%20Name))
    (else
      (CallFunction|LoadGame))))

(event EventEndPlay
  (params (EndPlayReason :type EEndPlayReason%20Enum :default "Destroyed"))
  ;[1 1 1] Save game at any end of play, either level transition or otherwise
  (CallFunction|SaveGame))

(fn ConstructionScript)

(fn SaveGame
  ;[1 1 1] Save game
  (bind _returnvalue (SaveGame|CreateSaveGameObject "/Game/Blueprints/Player/GM_Bogged_SaveGame.GM_Bogged_SaveGame_C"))
  (bind _output_get (Variables|Default|SetSaveRef _returnvalue))
  (Variables|/Game/Blueprints/Player/GM_Bogged_SaveGame.GM_Bogged_SaveGame_C|SetNewScore _output_get (+ (Variables|Default|GetNewScore) (Variables|/Game/Blueprints/Player/GM_Bogged_SaveGame.GM_Bogged_SaveGame_C|GetNewScore _output_get)))
  (SaveGame|SaveGametoSlot (Variables|Default|GetSaveRef) (Variables|Default|GetSave%20Slot%20Name)))

(fn LoadGame
  ;[1 1 1] Load Game
  (bind _returnvalue (SaveGame|DoesSaveGameExist (Variables|Default|GetSave%20Slot%20Name)))
  (if _returnvalue
    (Utilities|FlowControl|Sequence
      (:then_0
        (Utilities|FlowControl|DoOnce false :!label _label
          (:Completed
            (Development|PrintString "Hello")
            (bind _returnvalue_2 (SaveGame|LoadGamefromSlot (Variables|Default|GetSave%20Slot%20Name)))
            (bind _asgm_bogged_save_game (Utilities|Casting|CastToGM_Bogged_SaveGame _returnvalue_2))
            (Variables|Default|SetNewScore (Variables|/Game/Blueprints/Player/GM_Bogged_SaveGame.GM_Bogged_SaveGame_C|GetNewScore _asgm_bogged_save_game))
            (Development|PrintString (Variables|Default|GetSave%20Slot%20Name)))))
      (:then_1
        (goto _label Reset)))
    (else
      (CallFunction|SaveGame))))

(fn UpdateGMScore
  (params (PlayerScore :type Integer))
  ;[1 1 1] Update the score when we kill a root
  (if (not (Variables|Default|GetStopScoring))
    (Variables|Default|SetNewScore (+ (Variables|Default|GetNewScore) PlayerScore))))