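; BP_WallBuilder is an editor-built wall actor that lays out a straight row of repeated wall segments.
; Its construction script adds one InstancedStaticMesh instance per WallSegments count, offset along local X at a hard-coded 400-unit spacing.
; ChosenMaterial is applied to the instanced mesh's first material slot inside the loop.
; The event graph holds only disabled stub events, so it has no runtime logic.
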(event EventBeginPlay)

(event Collision|EventActorBeginOverlap
  (params (OtherActor :type Actor%20Object%20Reference)))

(event EventTick
  (params (DeltaSeconds :type Float%20%28single-precision%29)))

(fn ConstructionScript
  ;[1 1 1] Wall Section Script
  ;;[0.5239 0.92 1] Subtracts -1 from Index for the desired amount of segments
  (for _index (range 0 (- (Variables|Default|GetWall_Segments) 1))
    ;;[0.4947 0.8794 1] Create Segment
    (Components|InstancedStaticMesh|AddInstance (Variables|Default|GetInstancedStaticMesh) (Math|Transform|MakeTransform (Math|Vector|MakeVector (Math|Conversions|ToFloat(Integer) (* _index 400)) 0.0 0.0)) false)
    (Rendering|Material|SetMaterial (Variables|Default|GetInstancedStaticMesh) 0 (Variables|Default|GetChosenMaterial))))